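; BP_Door is a door actor that swings its static mesh open and closed through OpenDoor and CloseDoor events.
; BeginPlay stores the mesh's starting world rotation, and a timeline drives a yaw offset that is combined with it on each update.
; OpenDoor plays the timeline forward and CloseDoor reverses it.
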(event `self.ReceiveBeginPlay`
  (set `self.defRotation` (`SceneComponent.K2_GetComponentRotation` (`self.StaticMesh`))))

(event `OpenDoor`
  (bind (_direction _zaxis) (`Timeline|DoorTimeline` :!label _label)
    (:`Update`
      (`SceneComponent.K2_SetWorldRotation` (`self.StaticMesh`) (`KismetMathLibrary.ComposeRotators` (`KismetMathLibrary.MakeRotator` 0.0 0.0 _zaxis) (`self.defRotation`)) false false))))

(event `CloseDoor`
  (goto _label :!via `Reverse`))

(fn `UserConstructionScript`)